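; HeroBP is the player character, with tank-style axis movement, click-to-place pointing and a health pool.
; BeginPlay shows the cursor and spawns a MousePointBP marker, which left clicks move to the traced point under the cursor.
; The forward axis moves along the capsule's facing, while the right axis yaws the actor.
; Demage subtracts from Hp, and Tick restarts the level by console command once it is depleted.
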(event EventBeginPlay
  (bind _returnvalue (Game|SpawnActorfromClass "/Game/UI/MousePointBP.MousePointBP_C" (Math|Conversions|ToTransform(Vector) (Transformation|GetActorLocation)) "Undefined" 0 0))
  (Variables|Default|SetMouseClickPoint _returnvalue)
  (Variables|/Script/Engine.PlayerController|SetbShowMouseCursor (Game|GetPlayerController 0) true)
  (Variables|Default|Sethp 1e+02))

(event Collision|EventActorBeginOverlap
  (params (OtherActor :type Actor%20Object%20Reference)))

(event EventTick
  (params (DeltaSeconds :type Float%20%28single-precision%29))
  (if (<= (Variables|Default|Gethp) 0.0)
    (Development|ExecuteConsoleCommand "restartlevel")))

(event Input|ActionEvents|InputActionLeftMouseClicked
  (params (Key :type Key%20Structure :default "AnyKey"))
  (:Pressed
    (Transformation|SetActorLocation (Variables|Default|GetMouseClickPoint) (.Location (Collision|BreakHitResult (.HitResult (Game|Player|GetHitResultUnderCursorbyChannel (Game|GetPlayerController 0) "TraceTypeQuery1" true)))) false false)))

(event Input|AxisEvents|InputAxismoveForword
  (params (AxisValue :type Float%20%28single-precision%29))
  (Pawn|Input|AddMovementInput (Math|Vector|GetForwardVector (Variables|Collision|GetCapsuleComponent)) AxisValue false))

(event Input|AxisEvents|InputAxismoveRight
  (params (AxisValue :type Float%20%28single-precision%29))
  (Transformation|AddActorLocalRotation (Math|Rotator|MakeRotator 0.0 0.0 (* AxisValue -1.0)) false false))

(fn ConstructionScript)

(fn Demage
  (params (val :type Float%20%28single-precision%29))
  (Variables|Default|Sethp (- (Variables|Default|Gethp) val)))